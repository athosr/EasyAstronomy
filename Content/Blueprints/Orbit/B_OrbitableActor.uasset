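; Orbitable actor that circles a target actor on the horizontal plane while spinning its sphere mesh.
; Tick accumulates a signed, delta-scaled angle, and RotateActorAroundPoint offsets the actor by a rotated radius vector from the target, or from its BeginPlay location without one.
; The sphere's yaw spin is added per frame, so it is frame-rate dependent.
; An optional debug line connects orbit center and actor.
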(event EventBeginPlay
  ;[1 1 1] Sets the start location of the object
  (Variables|Default|SetInitLocation (Transformation|GetActorLocation)))

(event Collision|EventActorBeginOverlap
  (params (OtherActor :type Actor%20Object%20Reference)))

(event EventTick
  (params (DeltaSeconds :type Float%20%28single-precision%29))
  ;[1 1 1] Rotates the actor based on the transform of another actor
  (Variables|Default|SetCurrentRotation (+ (Variables|Default|GetCurrentRotation) (* (* (Variables|Default|GetRotationSpeed) DeltaSeconds) (select (Variables|Default|GetClockwise) -1.0 1.0))))
  (bind _newlocation (CallFunction|RotateActorAroundPoint self (Variables|Default|GetTargetActor) (Variables|Default|GetInitLocation) (Variables|Default|GetRadius) (Variables|Default|GetStartingAngle) (Variables|Default|GetCurrentRotation)))
  ;[1 1 1] Self rotation on actor
  (Transformation|SetWorldRotation (Variables|Default|GetSphere) (Math|Rotator|MakeRotator 0.0 0.0 (+ (.yaw (Transformation|GetWorldRotation (Variables|Default|GetSphere))) (Variables|Default|GetSelfRotationSpeed))) false false)
  ;[1 1 1] Debug Options
  (if (Variables|Default|GetDrawDebug)
    (Rendering|Debug|DrawDebugLine _newlocation (Transformation|GetActorLocation) (Variables|Default|GetTraceColor) 0.1 5.0)))

(fn ConstructionScript)

(fn RotateActorAroundPoint
  (params (ActorToRotate :type Actor%20Object%20Reference) (TargetActor :type Actor%20Object%20Reference) (TargetLocation :type Vector) (Radius :type Float%20%28single-precision%29) (Angle :type Float%20%28single-precision%29) (RotationRate :type Float%20%28single-precision%29))
  (LocalVariables|SetLActorToRotate ActorToRotate)
  (LocalVariables|SetLTargetActor TargetActor)
  (LocalVariables|SetLLocation TargetLocation)
  (LocalVariables|SetLRadius Radius)
  (LocalVariables|SetLAngle Angle)
  (LocalVariables|SetLRate RotationRate)
  (Utilities|IsValid (LocalVariables|GetLTargetActor)
    (:Is%20Valid
      (bind _output_get (LocalVariables|SetLLocation (Transformation|GetActorLocation (LocalVariables|GetLTargetActor)))))
    (:Is%20Not%20Valid
      _))
  (Transformation|SetActorLocation (LocalVariables|GetLActorToRotate) (+ _output_get (Math|Vector|RotateVectorAroundAxis (Math|Vector|MakeVector (LocalVariables|GetLRadius) 0.0 0.0) (+ (LocalVariables|GetLAngle) (LocalVariables|GetLRate)) "0, 0,1.000000")) false false)
  (return (LocalVariables|GetLLocation)))